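; Granular synth sound actor that plays a sound source with grain behavior driven by the player pawn's distance.
; Each tick maps distance to an Intensity value, optionally curve-shaped, which blends grain duration, rate, volume, pitch and pan ranges, and randomized playhead position.
; An optional curve adjusts tick interval by distance against attenuation falloff.
; Construction retriggers the note after a short delay; debug mode draws range spheres and prints state.
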(event `NoteOnAfterConstrScript`
  (bind _granularsynth (`self.GranularSynth`))
  ;[1 1 1] Note On from Construction Script, triggers when you tweak any values in runtime
  (`KismetSystemLibrary.Delay` 0.2)
  (`GranularSynth.SetSoundWave` _granularsynth (`self.SoundSource`))
  (`GranularSynth.NoteOn` _granularsynth (`self.Note`) (`self.Velocity`) (`self.Duration`)))

(event `self.ReceiveBeginPlay`
  (bind _soundsource (`self.SoundSource`))
  (bind _granularsynth (`self.GranularSynth`))
  ;[1 1 1] Setup
  (`/Engine/EditorBlueprintResources/StandardMacros.IsValid` _soundsource
    (:`Is Valid`
      (`/Engine/EditorBlueprintResources/StandardMacros.IsValid` (`self.Attenuation`)
        (:`Is Valid`
          _)
        (:`Is Not Valid`
          (`KismetSystemLibrary.PrintString` "No Attenuation Set - Might be problematic!")))
      ;;[1 1 1] SoundSource
      (`GranularSynth.SetSoundWave` _granularsynth _soundsource)
      (`/Engine/EditorBlueprintResources/StandardMacros.IsValid` _granularsynth
        (:`Is Valid`
          ;;[1 1 1] Start & NoteOn
          (`GranularSynth.NoteOn` _granularsynth (`self.Note`) (`self.Velocity`) (`self.Duration`)))
        (:`Is Not Valid`
          (`KismetSystemLibrary.PrintString` "SynthNotValid"))))
    (:`Is Not Valid`
      (`KismetSystemLibrary.PrintString` "No Sound Source Set! Problematic!"))))

(event `self.ReceiveTick`
  (params (DeltaSeconds :type "Float (single-precision)"))
  ;[1 1 1] Event Tick
  (`/Engine/EditorBlueprintResources/StandardMacros.IsValid` (`self.SoundSource`)
    (:`Is Valid`
      (set `self.TimeDelta` DeltaSeconds)
      (`self.ActorTickInterval`)
      (`self.UpdateSynth`)
      (`self.SynthDebug`))
    (:`Is Not Valid`
      (`/Engine/EditorBlueprintResources/StandardMacros.DoOnce` false
        (:`Completed`
          (`KismetSystemLibrary.PrintString` "No Sound Source Set! Problematic!"))))))

(event `UpdateSynth`
  (bind _returnvalue (`KismetMathLibrary.MapRangeClamped` (`self.PlayerDistance`) (`self.Range_Close`) (`self.Range_Far`) (`self.Intensity_Max`) (`self.Intensity_Min`)))
  ;[1 1 1] UpdateSynth
  (set `self.PlayerDistance` (`self.GetDistanceTo` (`GameplayStatics.GetPlayerPawn` 0)))
  (set `self.SynthTickRate` (/ 1.0 (`self.SynthUpdatePerSec`)))
  (if (`self.UseCurveForIntensityMapping`)
    (`/Engine/EditorBlueprintResources/StandardMacros.IsValid` (`self.Range2IntensityCurve`)
      (:`Is Valid`
        (set `self.Intensity` (`KismetMathLibrary.FMax` (`self.CurveMacro` _returnvalue (`self.Range2IntensityCurve`)))))
      (:`Is Not Valid`
        (set `self.Intensity` (`KismetMathLibrary.FMax` _returnvalue) :!label _label)))
    (else
      (goto _label)))
  (`self.SetGrainSettings`)
  (`self.SetPlaybackSettings_DistanceBased`)
  (`self.Set_ASR_Envelope`))

(fn `ActorTickInterval`
  (bind _actortickcurve (`self.ActorTickCurve`))
  (bind (_attenuation_battenuate _attenuation_bspatialize _attenuation_battenuatewithlpf _attenuation_benablelistenerfocus _attenuation_benablefocusinterpolation _attenuation_benableocclusion _attenuation_busecomplexcollisionforocclusion _attenuation_benablereverbsend _attenuation_benablepriorityattenuation _attenuation_bapplynormalizationtostereosounds _attenuation_benablelogfrequencyscaling _attenuation_benablesubmixsends _attenuation_spatializationalgorithm _attenuation_binauralradius _attenuation_absorptionmethod _attenuation_occlusiontracechannel _attenuation_reverbsendmethod _attenuation_priorityattenuationmethod _attenuation_omniradius _attenuation_stereospread _attenuation_lpfradiusmin _attenuation_lpfradiusmax _attenuation_customlowpassairabsorptioncurve _attenuation_customhighpassairabsorptioncurve _attenuation_lpffrequencyatmin _attenuation_lpffrequencyatmax _attenuation_hpffrequencyatmin _attenuation_hpffrequencyatmax _attenuation_focusazimuth _attenuation_nonfocusazimuth _attenuation_focusdistancescale _attenuation_nonfocusdistancescale _attenuation_focuspriorityscale _attenuation_nonfocuspriorityscale _attenuation_focusvolumeattenuation _attenuation_nonfocusvolumeattenuation _attenuation_focusattackinterpspeed _attenuation_focusreleaseinterpspeed _attenuation_occlusionlowpassfilterfrequency _attenuation_occlusionvolumeattenuation _attenuation_occlusioninterpolationtime _attenuation_reverbwetlevelmin _attenuation_reverbwetlevelmax _attenuation_reverbdistancemin _attenuation_reverbdistancemax _attenuation_manualreverbsendlevel _attenuation_customreverbsendcurve _attenuation_submixsendsettings _attenuation_priorityattenuationmin _attenuation_priorityattenuationmax _attenuation_priorityattenuationdistancemin _attenuation_priorityattenuationdistancemax _attenuation_manualpriorityattenuation _attenuation_custompriorityattenuationcurve _attenuation_pluginsettings _attenuation_distancealgorithm _attenuation_attenuationshape _attenuation_dbattenuationatmax _attenuation_falloffmode _attenuation_attenuationshapeextents _attenuation_coneoffset _attenuation_falloffdistance) (break `SoundAttenuationSettings` (`SoundAttenuation.Attenuation` (`self.Attenuation`))))
  (if (`self.UseCurveForActorTick`)
    (`/Engine/EditorBlueprintResources/StandardMacros.IsValid` (`self.Attenuation`)
      (:`Is Valid`
        (`/Engine/EditorBlueprintResources/StandardMacros.IsValid` _actortickcurve
          (:`Is Valid`
            (`self.SetActorTickInterval` (`KismetMathLibrary.FMin` (/ 1.0 (* (`self.SynthUpdatePerSec`) (`KismetMathLibrary.FClamp` (`CurveFloat.GetFloatValue` _actortickcurve (`KismetMathLibrary.MapRangeClamped` (`self.PlayerDistance`) 200.0 (* _attenuation_falloffdistance 1.2) 1.0))))) 0.5)))
          (:`Is Not Valid`
            _)))
      (:`Is Not Valid`
        _)))
  (return))

(fn `GrainSynthDebug`
  (bind _granularsynth (`self.GranularSynth`))
  (`KismetSystemLibrary.PrintString` (`KismetStringLibrary.Concat_StrStr` "IsPlaying:" (`KismetStringLibrary.Conv_BoolToString` (`SynthComponent.IsPlaying` _granularsynth)) " - " "IsLoaded:" (`KismetStringLibrary.Conv_BoolToString` (`GranularSynth.IsLoaded` _granularsynth)) " - " "CurrentPlayheadTime" (`KismetStringLibrary.Conv_DoubleToString` (`self.PlayHeadPos_Sec`)) " - " "PlayheadOffsetPerc:" (`KismetStringLibrary.Conv_DoubleToString` (`self.PlayHeadOffsetPerc`))))
  (`KismetSystemLibrary.PrintString` (`KismetStringLibrary.Conv_DoubleToString` (`self.Intensity`))))

(fn `Set_ASR_Envelope`
  (bind _granularsynth (`self.GranularSynth`))
  ;[1 1 1] ASR Envelope
  (`GranularSynth.SetAttackTime` _granularsynth (`self.AttackTime_ms`))
  (`GranularSynth.SetSustainGain` _granularsynth (`self.SustainGain`))
  (`GranularSynth.SetReleaseTimeMsec` _granularsynth (`self.ReleaseTime_ms`))
  (return))

(fn `SetGrainSettings`
  (bind _granularsynth (`self.GranularSynth`))
  (bind _returnvalue (`KismetMathLibrary.RandomFloatInRange` (`self.GrainsPerSec_Rand_Min`) (`self.GrainsPerSec_Rand_Max`)))
  (`GranularSynth.SetGrainEnvelopeType` _granularsynth (`self.EnvelopeType`))
  (`GranularSynth.SetGrainDuration` _granularsynth (`KismetMathLibrary.Lerp` (`self.GrainDuration_Min`) (`self.GrainDuration_Max`) (`self.Intensity`)) (`KismetMathLibrary.Conv_VectorToVector2D` (`KismetMathLibrary.VLerp` (`KismetMathLibrary.Conv_Vector2DToVector` (`self.Duration_Range_Min`)) (`KismetMathLibrary.Conv_Vector2DToVector` (`self.Duration_Range_Max`)) (`self.Intensity`))))
  (bind _output_get (set `self.GrainsPerSecond` (+ (`KismetMathLibrary.RandomFloatInRange` (* _returnvalue -1.0) _returnvalue) (`KismetMathLibrary.Lerp` (`self.GrainsPerSecond_Min`) (`self.GrainsPerSecond_Max`) (`self.Intensity`)))))
  (`GranularSynth.SetGrainsPerSecond` _granularsynth _output_get)
  (`GranularSynth.SetGrainVolume` _granularsynth (* (`KismetMathLibrary.Lerp` (`self.GrainVolume_Min`) (`self.GrainVolume_Max`) (`self.Intensity`)) (`self.SynthVolume`)) (`KismetMathLibrary.Conv_VectorToVector2D` (`KismetMathLibrary.VLerp` (`KismetMathLibrary.Conv_Vector2DToVector` (`self.GrainVolume_Range_Min`)) (`KismetMathLibrary.Conv_Vector2DToVector` (`self.GrainVolume_Range_Max`)) (`self.Intensity`))))
  (`GranularSynth.SetGrainProbability` _granularsynth (`self.InGrainProbability`))
  (`GranularSynth.SetGrainPitch` _granularsynth (`self.GrainBasePitch`) (`KismetMathLibrary.Conv_VectorToVector2D` (`KismetMathLibrary.VLerp` (`KismetMathLibrary.Conv_Vector2DToVector` (`self.GrainPitch_Range_Min`)) (`KismetMathLibrary.Conv_Vector2DToVector` (`self.GrainPitch_Range_Max`)) (`self.Intensity`))))
  (`GranularSynth.SetGrainPan` _granularsynth (`self.BasePan`) (`KismetMathLibrary.Conv_VectorToVector2D` (`KismetMathLibrary.VLerp` (`KismetMathLibrary.Conv_Vector2DToVector` (`self.GrainPan_RangeMin`)) (`KismetMathLibrary.Conv_Vector2DToVector` (`self.GrainPan_RangeMax`)) (`self.Intensity`))))
  (return))

(fn `SetPlaybackSettings_DistanceBased`
  (bind _granularsynth (`self.GranularSynth`))
  (bind _returnvalue (`KismetMathLibrary.Lerp` (`self.PlayHeadRandPos_Min`) (`self.PlayHeadRandPos_Max`) (`self.Intensity`)))
  (bind _returnvalue_2 (`KismetMathLibrary.RandomFloatInRange` (* _returnvalue -1.0) _returnvalue))
  (bind _returnvalue_3 (+ (`KismetMathLibrary.Lerp` (`self.PlayheadPos_Min_%`) (`self.PlayHeadPos_Max_%`) (`self.Intensity`)) _returnvalue_2))
  (`GranularSynth.SetScrubMode` _granularsynth (`self.EnableScrubMode`))
  (bind _output_get (set `self.PlayHeadPos_Sec` (* (`SoundBase.Duration` (`self.SoundSource`)) (/ _returnvalue_3 100.0))))
  (`GranularSynth.SetPlayheadTime` _granularsynth _output_get (`self.PlayHeadLerpTime_Sec`) (`self.SeekType`))
  (`GranularSynth.SetPlaybackSpeed` _granularsynth (`self.PlaybackSpeed`))
  (set `self.PlayHeadPos_Percent` _returnvalue_3)
  (set `self.PlayHeadOffsetPerc` _returnvalue_2)
  (return))

(fn `SynthDebug`
  (bind _timedelta (`self.TimeDelta`))
  (bind _returnvalue (`SceneComponent.K2_GetComponentLocation` (`self.GranularSynth`)))
  (bind _returnvalue_2 (* _timedelta 2.0))
  (if (`self.Debug`)
    (`KismetSystemLibrary.PrintString` (`KismetStringLibrary.Concat_StrStr` (`KismetSystemLibrary.GetDisplayName` (`ActorComponent.GetOwner` (`self.GranularSynth`))) (`KismetStringLibrary.Concat_StrStr` "  Distance " (`KismetStringLibrary.Conv_DoubleToString` (`self.GetDistanceTo` (`GameplayStatics.GetPlayerPawn` 0)))) (`KismetStringLibrary.Concat_StrStr` "  Intens " (`KismetStringLibrary.Conv_DoubleToString` (`self.Intensity`))) (`KismetStringLibrary.Concat_StrStr` "  PlayheadPosPercent " (`KismetStringLibrary.Conv_DoubleToString` (`self.PlayHeadPos_Percent`))) (`KismetStringLibrary.Concat_StrStr` "  Tick Interval PerSec " (`KismetStringLibrary.Conv_DoubleToString` (/ 1.0 (`self.GetActorTickInterval`)))) (`KismetStringLibrary.Concat_StrStr` "  GrainsPerSecond " (`KismetStringLibrary.Conv_DoubleToString` (`self.GrainsPerSecond`)))) true false (struct :`G` 0.66 :`B` 1.0 :`A` 1.0) _timedelta)
    (`KismetSystemLibrary.DrawDebugSphere` _returnvalue (`self.Range_Far`) 12 (struct :`R` 0.442708 :`G` 0.442708 :`B` 0.442708 :`A` 1.0) _returnvalue_2)
    (`KismetSystemLibrary.DrawDebugSphere` _returnvalue (`self.Range_Close`) 12 (struct :`R` 1.0 :`G` 1.0 :`B` 1.0 :`A` 1.0) _returnvalue_2)
    (`KismetSystemLibrary.DrawDebugString` _returnvalue "Range To Intensity Sphere" null (struct :`R` 1.0 :`G` 1.0 :`B` 1.0 :`A` 1.0) _returnvalue_2)))

(fn `UserConstructionScript`
  (bind _attenuation (`self.Attenuation`))
  (`/Engine/EditorBlueprintResources/StandardMacros.IsValid` _attenuation
    (:`Is Valid`
      (set `SynthComponent.AttenuationSettings` _attenuation (`self.GranularSynth`))
      (`self.NoteOnAfterConstrScript`))
    (:`Is Not Valid`
      (`KismetSystemLibrary.PrintString` "Attenuation Not Valid!"))))